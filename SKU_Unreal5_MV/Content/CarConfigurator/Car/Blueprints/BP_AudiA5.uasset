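; BP_AudiA5 is the car configurator's Audi A5 convertible, combining a Control Rig with interior and exterior lighting effects.
; RigSetup snaps bones to pivot components, while SplineControl places the root along a spline and steers from a look-ahead point.
; Helpers ramp light intensities, assign dynamic LED materials, set warning lights and blend dial rotations.
; The roof switches between configurator and cinematic meshes, with material swaps hiding parts when open.
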(fn ConstructionScript)

(fn RigSetup
  (bind _controlrig (Variables|Default|GetControlRig))
  ;[1 1 1] For each RigPrep object, find the corresponding ControlRig bone. Snap the bone to the RigPrep object location
  (for _array_element (Components|GetChildrenComponents (Variables|Default|Getpivots1) true)
    (Class|ControlRigComponent|SetInitialBoneTransform _controlrig (Utilities|String|StringToName (Utilities|String|LeftChop (Utilities|GetObjectName _array_element) 1)) (Transformation|GetWorldTransform _array_element) "WorldSpace" true)
    (Class|ControlRigComponent|SetBoneTransform _controlrig (Utilities|String|StringToName (Utilities|String|LeftChop (Utilities|GetObjectName _array_element) 1)) (Transformation|GetWorldTransform _array_element) "WorldSpace" 1.0 true)))

(fn SplineControl
  (bind _splinedistance (Variables|Spline|GetSplineDistance))
  (bind _splineactor (Variables|Spline|GetSplineActor))
  (bind _returnvalue (Actor|GetComponentbyClass _splineactor "/Script/Engine.SplineComponent"))
  (bind _returnvalue_2 (Spline|GetTransformatDistanceAlongSpline _returnvalue _splinedistance "World" false))
  (if (Utilities|IsValid _splineactor)
    (Class|ControlRigComponent|SetControlTransform (Variables|Default|GetControlRig) "root_ctrl" (Math|Transform|ComposeTransforms (Math|Transform|MakeTransform (Math|Vector|MakeVector (Variables|Default|GetChassisOffset) 0.0 0.0)) _returnvalue_2) "WorldSpace")
    (Class|ControlRigComponent|SetControlFloat (Variables|Default|GetControlRig) "Steering_CTRL" (* (.y (Math|Transform|InverseTransformLocation _returnvalue_2 (.location (Spline|GetTransformatDistanceAlongSpline _returnvalue (+ _splinedistance (Variables|Spline|GetSplineSteerAhead)) "World" false)))) 1.0))))

(fn BlendControlRigInput
  (params (Control :type Name) (TargetRot :type Rotator) (IsOpen :type Boolean) (AnimationScale :type Float%20%28double-precision%29) (TargetPos :type Vector) (IsDoor? :type Boolean)))

(fn IncreaseLEDs
  (params (DT :type Float%20%28double-precision%29))
  (Utilities|FlowControl|Sequence
    (:then_0
      (Variables|LEDs|SetLEDDIntensity (Math|Float|Min(Float) (+ (* DT 2e+04) (Variables|LEDs|GetLEDDIntensity)) 2e+04)))
    (:then_1
      (Variables|LEDs|SetHMIIntensity (Math|Float|Min(Float) (+ (* DT 2e+03) (Variables|LEDs|GetHMIIntensity)) 3e+03)))
    (:then_2
      (Variables|LEDs|SetFrontLightIntensity (Math|Float|Min(Float) (+ (Variables|LEDs|GetFrontLightIntensity) 1e+03) 7.5e+04)))))

(fn DecreaseLEDs
  (params (DT :type Float%20%28double-precision%29))
  (Utilities|FlowControl|Sequence
    (:then_0
      (Variables|LEDs|SetLEDDIntensity (Math|Float|Max(Float) (- (Variables|LEDs|GetLEDDIntensity) (* DT 2e+04)) 0.0)))
    (:then_1
      (Variables|LEDs|SetHMIIntensity (Math|Float|Max(Float) (- (Variables|LEDs|GetHMIIntensity) (* DT 2e+03)) 0.0)))
    (:then_2
      (Variables|LEDs|SetFrontLightIntensity (Math|Float|Max(Float) (- (Variables|LEDs|GetFrontLightIntensity) 1e+03) 5e+02)))))

(fn AssignDynamicMaterials
  ;[1 1 1] Dashboard
  (Rendering|Material|SetMaterial (Variables|Default|GetSM_gaugeDisplay) 0 (Variables|LEDs|GetLEDDisplayDynamicMat))
  (Rendering|Material|SetMaterial (Variables|Default|GetSM_lightControls) 4 (Variables|LEDs|GetLEDWhiteDynamicMaterial))
  (Rendering|Material|SetMaterial (Variables|Default|GetSM_dialBack) 1 (Variables|LEDs|GetLEDWhiteDynamicMaterial))
  (Rendering|Material|SetMaterial (Variables|Default|GetSM_dialBack) 4 (Variables|LEDs|GetLEDRedDynamicMaterial))
  (Rendering|Material|SetMaterial (Variables|Default|GetSM_dialBack) 5 (Variables|LEDs|GetLEDYellow_Dynamic_Material))
  (Rendering|Material|SetMaterial (Variables|Default|GetSM_steeringwheel) 1 (Variables|LEDs|GetLEDWhiteDynamicMaterial))
  (Rendering|Material|SetMaterial (Variables|Default|GetSM_extraButtons) 3 (Variables|LEDs|GetLEDWhiteDynamicMaterial))
  ;[1 1 1] HMI
  (Rendering|Material|SetMaterial (Variables|Default|GetSM_HMI) 0 (Variables|LEDs|GetHMIDynamicMaterial))
  ;[1 1 1] Heating control
  (Rendering|Material|SetMaterial (Variables|Default|GetSM_heatingControl) 6 (Variables|LEDs|GetLEDRedDynamicMaterial))
  (Rendering|Material|SetMaterial (Variables|Default|GetSM_heatingControl) 8 (Variables|LEDs|GetLEDRedDynamicMaterial))
  (Rendering|Material|SetMaterial (Variables|Default|GetSM_heatingControl) 7 (Variables|LEDs|GetLEDClimateDynamicMaterial))
  (Rendering|Material|SetMaterial (Variables|Default|GetSM_heatingControl) 3 (Variables|LEDs|GetLEDClimateDynamicMaterial))
  (Rendering|Material|SetMaterial (Variables|Default|GetSM_heatingControl) 9 (Variables|LEDs|GetLEDBlueDynamicMaterial))
  ;[1 1 1] Speed and tach
  (Rendering|Material|SetMaterial (Variables|Default|GetSM_tachNeedle) 1 (Variables|LEDs|GetLEDRedDynamicMaterial))
  (Rendering|Material|SetMaterial (Variables|Default|GetSM_speedNeedle) 3 (Variables|LEDs|GetLEDRedDynamicMaterial))
  ;[1 1 1] Center console
  (Rendering|Material|SetMaterial (Variables|Default|GetSM_centerconsoleControl) 5 (Variables|LEDs|GetLEDWhiteDynamicMaterial))
  (Rendering|Material|SetMaterial (Variables|Default|GetSM_centerconsoleControl) 8 (Variables|LEDs|GetLEDWhiteDynamicMaterial))
  (Rendering|Material|SetMaterial (Variables|Default|GetSM_centerconsoleControl) 12 (Variables|LEDs|GetLEDRedDynamicMaterial))
  ;[1 1 1] Front lights
  (Rendering|Material|SetMaterial (Variables|Default|GetSM_Iheadlightglass) 0 (Variables|LEDs|GetLightGlassDynamicMat))
  (Rendering|Material|SetMaterial (Variables|Default|GetSM_headlightBrowLight) 0 (Variables|LEDs|GetLightBrowsDynamicMaterial))
  ;[1 1 1] taillights
  (Rendering|Material|SetMaterial (Variables|Default|GetSM_Brakeinnerglass) 0 (Variables|LEDs|GetTailLightsDynamicMaterial)))

(fn UpdateAniminEditor
  (Components|SkeletalMesh|SetUpdateAnimationinEditor (Variables|Default|GetConvertibleTop) true))

(fn SwitchTopVisible
  (bind _convertibletopcine (Variables|Default|GetConvertibleTopCine))
  (bind _convertibletop (Variables|Default|GetConvertibleTop))
  (if (Variables|Default|GetCarConfiguratorMode)
    (Rendering|SetVisibility _convertibletop true true)
    (Rendering|SetVisibility _convertibletopcine false true)
    (else
      (Rendering|SetVisibility _convertibletopcine true true)
      (Rendering|SetVisibility _convertibletop false true))))

(fn HideinTrunk
  (if (Variables|SoftTopAnimation|GetisTopOpen)
    (Rendering|Material|SetMaterial (Variables|Default|GetConvertibleTop) 15 "/Game/CarConfigurator/Car/ConvertibleTop/M_Hiding.M_Hiding")
    (Rendering|Material|SetMaterial (Variables|Default|GetConvertibleTop) 31 "/Game/CarConfigurator/Car/ConvertibleTop/M_Hiding.M_Hiding")
    (Rendering|Material|SetMaterial (Variables|Default|GetConvertibleTop) 7 "/Game/CarConfigurator/Car/ConvertibleTop/M_Hiding.M_Hiding")
    (Rendering|Material|SetMaterial (Variables|Default|GetConvertibleTop) 17 "/Game/CarConfigurator/Car/ConvertibleTop/M_Hiding.M_Hiding")
    (Rendering|Material|SetMaterial (Variables|Default|GetConvertibleTop) 27 "/Game/CarConfigurator/Car/ConvertibleTop/M_Hiding.M_Hiding")))

(fn ShowinTrunk
  (if (Variables|SoftTopAnimation|GetisTopOpen)
    (Rendering|Material|SetMaterial (Variables|Default|GetConvertibleTop) 15 "/Game/CarConfigurator/Car/ConvertibleTop/MI_TextilePlain_Int.MI_TextilePlain_Int")
    (Rendering|Material|SetMaterial (Variables|Default|GetConvertibleTop) 31 "/Game/CarConfigurator/Car/ConvertibleTop/MI_Glass_Convertible.MI_Glass_Convertible")
    (Rendering|Material|SetMaterial (Variables|Default|GetConvertibleTop) 7 "/Game/CarConfigurator/Car/ConvertibleTop/MI_TextilePlain_Int.MI_TextilePlain_Int")
    (Rendering|Material|SetMaterial (Variables|Default|GetConvertibleTop) 17 "/Game/CarConfigurator/Car/ConvertibleTop/MI_Metal_Painted.MI_Metal_Painted")
    (Rendering|Material|SetMaterial (Variables|Default|GetConvertibleTop) 27 "/Game/CarConfigurator/Car/ConvertibleTop/MI_Metal_Painted.MI_Metal_Painted")))

(fn BlendControlRigInputDials
  (params (Control :type Name) (TargetRot :type Rotator) (IsOpen :type Boolean) (AnimationScale :type Float%20%28double-precision%29) (TargetPos :type Vector))
  ;[1 1 1] Open Animation
  (Class|ControlRigComponent|SetControlTransform (Variables|Default|GetControlRig) Control (Math|Transform|MakeTransform "0, 0, 0" (Math|Rotator|MakeRotator (Math|Float|Lerp (.roll (Class|ControlRigComponent|GetControlRotator (Variables|Default|GetControlRig) Control "LocalSpace")) (.roll TargetRot) (* (Utilities|Time|GetWorldDeltaSeconds) AnimationScale)) 0.0 0.0) "1.000000,1.000000,1.000000") "LocalSpace"))

(fn SetWarningLights
  (params (InputVal :type Float%20%28double-precision%29))
  (bind _output_get (LocalVariables|SetInputValue InputVal))
  (if (Math|Boolean|ORBoolean (== _output_get 1.0) (== _output_get 4.0) (== _output_get 8.0))
    (LocalVariables|SetMaterialValue "/Game/CarConfigurator/Shared/Materials/MI_LED_YellowWarning.MI_LED_YellowWarning")
    (else
      (LocalVariables|SetMaterialValue "/Game/CarConfigurator/Shared/Materials/MI_LED_RedWarning.MI_LED_RedWarning")))
  (if (< (LocalVariables|GetInputValue) 0.0)
    (Rendering|Material|SetMaterial (Variables|Default|GetSM_WarningLights) (- (Math|Float|Truncate (* (LocalVariables|GetInputValue) -1.0)) 1) "/Game/References/AutomotiveMats/Materials/Interior/Plastic/MI_Plastic_Smooth_Grey.MI_Plastic_Smooth_Grey")
    (else
      (Rendering|Material|SetMaterial (Variables|Default|GetSM_WarningLights) (- (Math|Float|Truncate (LocalVariables|GetInputValue)) 1) (LocalVariables|GetMaterialValue)))))